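; CheekyCharacter is the first-person player character, handling movement, smoothed look, leaning, zoom, jumping and HUD creation.
; A looping 0.1-second timer derives walk, sneak or run state, updates stamina with exhaustion cooldown, and sets speed as scaled movement input against a fixed run-speed maximum.
; Custom crouch animates capsule height by timeline and retries a sphere trace before standing.
; Components handle health, footsteps and leaning, while PlayerSettingsManager tunes look and headbob shake.
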(event `self.ReceiveBeginPlay`
  (`KismetSystemLibrary.K2_SetTimerDelegate` (delegate `PlayerUpdates`) 0.1 true)
  (`self.PlayCameraShake` "/Game/CheekyFPS/Blueprints/CameraManager/CamShakes/CamShake_Idle.CamShake_Idle_C")
  ;[1 1 1] Set MaxWalkSpeed to = Run Speed
  (set `CharacterMovementComponent.MaxWalkSpeed` (`self.BaseRunSpeed`) (`self.CharacterMovement`))
  ;[1 1 1] Create HUD
  (bind _returnvalue (`|CreateWidget` "/Game/CheekyFPS/Blueprints/WBP_HUD.WBP_HUD_C" null self))
  (`UserWidget.AddToViewport` _returnvalue 0))

(event `PlayerUpdates`
  ;[0.05719 0.2929 1] Things to run frequently - but not tick
  ;;[1 0.4446 0.1392] Movement
  (`self.CalculateMovementState`)
  (`self.CalculatePlayerSpeed`)
  (`self.UpdateStamina`))

(event `self.OnLanded`
  (params (Hit :type "HitResult Structure (by ref)"))
  ;[0 0.3626 1] Fall Damage - for some reason this can't be bound in a component
  ;
  ; This also ripples back to generate footstep events
  (`/Game/CheekyFPS/Blueprints/Health/CheekyHealthComponent.OnLanded` (`self.HealthComponent`)))

(event `InputAction|[CHEEKY]Jump`
  (params (Key :type "Key Structure"))
  ;[0.1944 1 0.4592] Movement Actions
  (:`Pressed`
    (`self.JumpStart`))
  (:`Released`
    (`self.JumpEnd`)))

(event `InputAxis|[FPS]MoveForward`
  (params (AxisValue :type "Float (single-precision)"))
  ;[0.1175 0.1248 1] Movement
  (`self.MoveForwardInput` AxisValue))

(event `InputAxis|[FPS]MoveRight`
  (params (AxisValue :type "Float (single-precision)"))
  ;[0.1175 0.1248 1] Movement
  (`self.MoveRightInput` AxisValue))

(event `InputAction|[CHEEKY]Crouch`
  (params (Key :type "Key Structure"))
  ;[0.1944 1 0.4592] Movement Actions
  (:`Pressed`
    (`self.BeginCrouch`))
  (:`Released`
    (`self.EndCrouch`)))

(event `InputAction|[CHEEKY]Sneak`
  (params (Key :type "Key Structure"))
  ;[0.1944 1 0.4592] Movement Actions
  (:`Pressed`
    (set `self.bIsTryingToSneak` true))
  (:`Released`
    (set `self.bIsTryingToSneak` false)))

(event `InputAxisKey|MouseY`
  (params (AxisValue :type "Float (single-precision)"))
  ;[1 0.1188 0.6025] Mouselook
  (`self.LookVertical` (* AxisValue -1.0)))

(event `InputAction|[CHEEKY]Run`
  (params (Key :type "Key Structure"))
  ;[0.1944 1 0.4592] Movement Actions
  (:`Pressed`
    (set `self.bIsTryingToRun` true))
  (:`Released`
    (set `self.bIsTryingToRun` false)))

(event `InputAxisKey|MouseX`
  (params (AxisValue :type "Float (single-precision)"))
  ;[1 0.1188 0.6025] Mouselook
  (`self.LookHorizontal` AxisValue))

(event `InputAction|[CHEEKY]Zoom`
  (params (Key :type "Key Structure"))
  ;[1 0.3846 0] Zoom
  (:`Pressed`
    (`self.ZoomView` true))
  (:`Released`
    (`self.ZoomView` false)))

(event `InputAxisKey|Gamepad_RightY`
  (params (AxisValue :type "Float (single-precision)"))
  ;[1 0.1357 0.3162] Gamepad Look
  (`self.LookVertical` AxisValue true))

(event `InputAxisKey|Gamepad_RightX`
  (params (AxisValue :type "Float (single-precision)"))
  ;[1 0.1357 0.3162] Gamepad Look
  (`self.LookHorizontal` AxisValue true))

(event `InputAxis|[FPS]LeanRight`
  (params (AxisValue :type "Float (single-precision)"))
  ;[0.1686 0.2777 1] Leaning
  (`/Game/CheekyFPS/Blueprints/CheekyLeanComponent.UpdateLeanFromAxis` (`self.LeanComponent`) AxisValue))

(event `MoveForwardInput`
  (params (Axis :type "Float (double-precision)"))
  ;[0.03282 0.338 1] Move Forward
  (`self.AddMovementInput` (`self.GetActorForwardVector`) (* Axis (`self.NormalisedMovementSpeed`) (select `bool` (< Axis 0.0) :`false` 1.0 :`true` (`self.BackwardsPenalty`)))))

(event `MoveRightInput`
  (params (Axis :type "Float (double-precision)"))
  ;[0.03282 0.338 1] Move Right
  (`self.AddMovementInput` (`self.GetActorRightVector`) (* Axis (`self.NormalisedMovementSpeed`) (`self.SidewaysPenalty`))))

(event `LookVertical`
  (params (Axis :type "Float (double-precision)") (bIsGamepad :type Boolean))
  (bind _playersettingsmanager (`self.PlayerSettingsManager`))
  ;[1 0.2764 0.6413] Look Vertical
  ;;[0.2562 0.541 1] Smooth Axis Input
  (bind _output_get (set `self.SmoothVerticalLook` (`KismetMathLibrary.FInterpTo` (`self.SmoothVerticalLook`) Axis (`GameplayStatics.GetWorldDeltaSeconds`) (`/Game/CheekyFPS/Blueprints/CheekyPlayerSettingsManager.GetLookSmooth` (`self.PlayerSettingsManager`) bIsGamepad))))
  ;;[1 0.3819 0.2215] Apply settings, apply to controller
  (`self.AddControllerPitchInput` (* _output_get (`KismetMathLibrary.SelectFloat` -1.0 1.0 (`/Game/CheekyFPS/Blueprints/CheekyPlayerSettingsManager.GetLookInvertY` _playersettingsmanager bIsGamepad)) (`/Game/CheekyFPS/Blueprints/CheekyPlayerSettingsManager.GetLookSensY` _playersettingsmanager bIsGamepad))))

(event `LookHorizontal`
  (params (Axis :type "Float (double-precision)") (bIsGamepad :type Boolean))
  (bind _playersettingsmanager (`self.PlayerSettingsManager`))
  ;[1 0.2764 0.6413] Look Horizontal
  ;;[0.2562 0.541 1] Smooth Axis Input
  (bind _output_get (set `self.SmoothHorizontalLook` (`KismetMathLibrary.FInterpTo` (`self.SmoothHorizontalLook`) Axis (`GameplayStatics.GetWorldDeltaSeconds`) (`/Game/CheekyFPS/Blueprints/CheekyPlayerSettingsManager.GetLookSmooth` (`self.PlayerSettingsManager`) bIsGamepad))))
  ;;[1 0.3819 0.2215] Apply settings, apply to controller
  (`self.AddControllerYawInput` (* _output_get (`KismetMathLibrary.SelectFloat` -1.0 1.0 (`/Game/CheekyFPS/Blueprints/CheekyPlayerSettingsManager.GetLookInvertY` _playersettingsmanager bIsGamepad)) (`/Game/CheekyFPS/Blueprints/CheekyPlayerSettingsManager.GetLookSensY` _playersettingsmanager bIsGamepad))))

(event `BeginCrouch`
  ;[1 0.6419 0] Crouching Logic - this avoid's Epic's implementation on the character as it's very basic
  (if (not (`self.bIsCrouching`))
    (set `self.bIsCrouching` true)
    (`self.PlayCameraShake` "/Game/CheekyFPS/Blueprints/CameraManager/CamShakes/CamShake_CrouchDown.CamShake_CrouchDown_C")
    (bind (_direction _animation) (`Timeline|CrouchTimeline` :!label _label)
      (:`Update`
        (`CapsuleComponent.SetCapsuleHalfHeight` (`self.CapsuleComponent`) (`KismetMathLibrary.Lerp` (`self.PlayerHalfHeight`) (`self.PlayerCrouchedHeight`) _animation) true)))))

(event `JumpStart`
  ;[1 0.0205 0.9536] Jump / Landing
  (`self.Jump`)
  (`/Game/CheekyFPS/Blueprints/Footsteps/CheekyFootstepComponent.PlayFootstep` (`self.FootstepComponent`) "NewEnumerator3" 1 1.0))

(event `JumpEnd`
  ;[1 0.0205 0.9536] Jump / Landing
  (`self.StopJumping`))

(event `EndCrouch`
  (bind _returnvalue (`SceneComponent.K2_GetComponentLocation` (`self.CapsuleComponent`)))
  ;[1 0.6419 0] Crouching Logic - this avoid's Epic's implementation on the character as it's very basic
  (bind (_outhit _returnvalue_2) (`KismetSystemLibrary.SphereTraceSingle` _returnvalue (+ _returnvalue (0.0 0.0 150.0)) 15.0 "TraceTypeQuery1" :!label _label_2))
  (if _returnvalue_2
    (`KismetSystemLibrary.Delay` 0.2)
    (goto _label_2)
    (else
      (set `self.bIsCrouching` false)
      (`self.PlayCameraShake` "/Game/CheekyFPS/Blueprints/CameraManager/CamShakes/CamShake_CrouchUp.CamShake_CrouchUp_C")
      (goto _label :!via `Reverse`))))

(event `self.HealthComponent.OnLandFootstep`
  (params (Volume :type "Float (single-precision)"))
  ;[1 0.0205 0.9536] Jump / Landing
  (`/Game/CheekyFPS/Blueprints/Footsteps/CheekyFootstepComponent.PlayFootstep` (`self.FootstepComponent`) "NewEnumerator5" 1 Volume))

(event `ZoomView`
  (params (bStart :type Boolean))
  ;[1 0.31 0.6422] Zoom / Focus Mode
  (if bStart
    (`/Engine/EditorBlueprintResources/StandardMacros.IsValid` (`self.CameraModifierZoom`)
      (:`Is Valid`
        _)
      (:`Is Not Valid`
        (bind _returnvalue (`PlayerCameraManager.AddNewCameraModifier` (`GameplayStatics.GetPlayerCameraManager` 0) "/Game/CheekyFPS/Blueprints/CameraManager/CamModifiers/CamModifier_InspectZoom.CamModifier_InspectZoom_C")) ; This should only happen the first time the player uses zoom
        (set `self.CameraModifierZoom` _returnvalue)))
    (`CameraModifier.EnableModifier` (`self.CameraModifierZoom`))
    (set `self.bIsInZoomMode` true)
    (else
      (`/Engine/EditorBlueprintResources/StandardMacros.IsValid` (`self.CameraModifierZoom`) :!label _label
        (:`Is Valid`
          (`CameraModifier.DisableModifier` (`self.CameraModifierZoom`) false)
          (set `self.bIsInZoomMode` false))
        (:`Is Not Valid`
          (set `self.bIsInZoomMode` false))))))

(event `EndZoom`
  ;[1 0.31 0.6422] Zoom / Focus Mode
  (goto _label))

(fn `CalculateMovementState`
  (locals (CurrentVelocity :type "Float (double-precision)") (CanPlayerRun :type Boolean))
  (bind _output_get (set `local.CurrentVelocity` (`KismetMathLibrary.VSize` (`CharacterMovementComponent.GetLastUpdateVelocity` (`self.CharacterMovement`)))))
  ;[1 1 1] This is generally useful for other systems
  (set `self.bIsPlayerMoving` (and (`NavMovementComponent.IsMovingOnGround` (`self.CharacterMovement`)) (not (`KismetMathLibrary.NearlyEqual_FloatFloat` _output_get 0.0 1.0))))
  ;[1 1 1] Can player run?
  (set `local.CanPlayerRun` (and (not (`self.bIsPlayStaminaOnCooldown`)) (> (`local.CurrentVelocity`) 100.0)))
  ;[1 1 1] Final movement state
  (set `self.MovementState` (select `bool` (and (`self.bIsTryingToRun`) (`local.CanPlayerRun`)) :`false` (select `bool` (`self.bIsTryingToSneak`) :`false` "NewEnumerator0" :`true` "NewEnumerator1" :!type "/Game/CheekyFPS/Blueprints/EMovementSpeeds Enum") :`true` "NewEnumerator2"))
  (return))

(fn `CalculatePlayerSpeed`
  (locals (MovementPenalties :type "Float (double-precision)" :default 1.0))
  (set `local.MovementPenalties` (* 1.0 (select `bool` (`self.bIsInZoomMode`) :`false` 1.0 :`true` (`self.ZoomPenalty`))))
  ;[1 1 1] Calculate Normalised Speed - this could be more efficient by precalculating values
  (set `self.NormalisedMovementSpeed` (* (select `bool` (`self.bIsCrouching`) :`false` (select `/Game/CheekyFPS/Blueprints/EMovementSpeeds` (`self.MovementState`) :`NewEnumerator0` (/ (`self.BaseWalkSpeed`) (`self.BaseRunSpeed`)) :`NewEnumerator1` (/ (`self.BaseSneakSpeed`) (`self.BaseRunSpeed`)) :`NewEnumerator2` 1.0) :`true` (/ (`self.BaseCrouchSpeed`) (`self.BaseRunSpeed`))) (`local.MovementPenalties`)))
  (return))

(fn `PlayCameraShake`
  (params (ShakeClass :type "CameraShake Class Reference") (Scale :type "Float (double-precision)" :default 1.0) (bIgnoreHeadbobSettings :type Boolean))
  (`PlayerCameraManager.PlayCameraShake` :`self` (`GameplayStatics.GetPlayerCameraManager` 0) :`ShakeClass` (`local.ShakeClass`) :`Scale` (select `bool` (`local.bIgnoreHeadbobSettings`) :`false` (* (`local.Scale`) (`/Game/CheekyFPS/Blueprints/CheekyPlayerSettingsManager.HeadbobScale` (`self.PlayerSettingsManager`))) :`true` (`local.Scale`)))
  (return))

(fn `UpdateStamina`
  (bind _output_get (set `self.Stamina` (`KismetMathLibrary.FClamp` (+ (`self.Stamina`) (/ (select `bool` (`self.bIsPlayerMoving`) :`false` 7.0 :`true` (select `/Game/CheekyFPS/Blueprints/EMovementSpeeds` (`self.MovementState`) :`NewEnumerator0` 4.0 :`NewEnumerator1` 6.0 :`NewEnumerator2` -10.0 :!type "Float (single-precision)")) 10.0)) 0.0 100.0)))
  ;[1 1 1] If stamina hits 0, enable cooldown
  (if (== _output_get 0.0)
    (set `self.bIsPlayStaminaOnCooldown` true)
    (return)
    (else
      ;[1 1 1] If stamina is above 20, make sure cooldown is off
      (if (>= _output_get (`self.StaminaCooldownThreshold`))
        (set `self.bIsPlayStaminaOnCooldown` false)
        (return)
        (else
          ;[1 1 1] Do not change stamina state
          (return))))))

(fn `UserConstructionScript`)