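; Scene component parented to a camera that procedurally sways the first-person weapon by rotating itself every tick.
; Pitch and yaw come from the clamped camera rotation delta since the last frame, while roll comes from the owner's velocity along the camera's right vector for a strafe lean.
; A weapon-down flag scales the sway and adds a downward pitch offset, and RInterpTo smooths the result.
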(event `self.ReceiveBeginPlay`
  ;[0 1 0.06347] Get a referecence to the parent camera
  (bind _ascamera_component (cast `CameraComponent` (`self.GetAttachParent`)))
  (set `self.ParentCamera` _ascamera_component)
  ;[0 1 0.7235] Get owning actor - we need this to detect when the player is strafing
  (set `self.OwningActor` (`self.GetOwner`)))

(event `self.ReceiveTick`
  (params (DeltaSeconds :type "Float (single-precision)"))
  ;[1 0.2888 0] Where the magic happens
  (`self.UpdateSway`))

(fn `SetWeaponDown`
  (params (bWeaponIsDown :type Boolean))
  (set `self.bWeaponIsDown` bWeaponIsDown)
  (return))

(fn `UpdateSway`
  (bind _horizontalswaycap (`self.HorizontalSwayCap`))
  (bind _verticalswaycap (`self.VerticalSwayCap`))
  (bind _returnvalue (`Actor.GetVelocity` (`self.OwningActor`)))
  (bind _returnvalue_2 (`KismetMathLibrary.MakeRotator` (* (`KismetMathLibrary.Dot_VectorVector` (`self.GetRightVector` (`self.ParentCamera`)) (`KismetMathLibrary.Normal` _returnvalue 0.1)) (* (`KismetMathLibrary.FClamp` (/ (`KismetMathLibrary.VSize` _returnvalue) 400.0)) (`self.StrafeRoll`))) (`KismetMathLibrary.FClamp` (* (.pitch (`KismetMathLibrary.NormalizedDeltaRotator` (`self.LastCameraRotation`) (`self.K2_GetComponentRotation` (`self.ParentCamera`)))) (`self.VerticalSwaySensitivity`)) (* _verticalswaycap -1.0) _verticalswaycap) (`KismetMathLibrary.FClamp` (* (.yaw (`KismetMathLibrary.NormalizedDeltaRotator` (`self.LastCameraRotation`) (`self.K2_GetComponentRotation` (`self.ParentCamera`)))) (`self.HorizontalSwaySensitivity`)) (* _horizontalswaycap -1.0) _horizontalswaycap)))
  ;[1 0.08798 0] Smooth it all out
  (bind _output_get (set `self.WeaponSway` (`KismetMathLibrary.RInterpTo` (`self.WeaponSway`) (select `bool` (`self.bWeaponIsDown`) :`false` _returnvalue_2 :`true` (`KismetMathLibrary.ComposeRotators` (* _returnvalue_2 (`self.ReduceSwayWhenWeaponDown`)) (`KismetMathLibrary.MakeRotator` 0.0 (`self.WeaponDownAmount`)))) (`GameplayStatics.GetWorldDeltaSeconds`) (`self.SwaySpeed`))))
  (`self.K2_SetRelativeRotation` _output_get)
  (set `self.LastCameraRotation` (`self.K2_GetComponentRotation` (`self.ParentCamera`)))
  (return))