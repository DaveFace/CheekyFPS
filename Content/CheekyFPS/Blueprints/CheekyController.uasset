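; Player controller for CheekyFPS that toggles the pause menu when Escape or P is pressed.
; Showing the menu pauses the game, creates a WBP_PauseMenu widget, binds its OnReturn event and switches to UI-only input with the cursor visible.
; Hiding it unpauses, restores game-only input, hides the cursor, closes the widget and clears the reference, whose validity serves as the toggle state.
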(event `Key|Escape`
  (params (Key :type "Key Structure"))
  ;[1 0 0.2597] Pause Menu
  (:`Pressed`
    (`/Engine/EditorBlueprintResources/StandardMacros.IsValid` (`self.PauseMenuWidget`) :!label _label
      (:`Is Valid`
        (`self.HidePauseMenu`))
      (:`Is Not Valid`
        (`self.ShowPauseMenu`)))))

(event `Key|P`
  (params (Key :type "Key Structure"))
  ;[1 0 0.2597] Pause Menu
  (:`Pressed`
    (goto _label)))

(fn `HidePauseMenu`
  (`GameplayStatics.SetGamePaused` false)
  (`WidgetBlueprintLibrary.SetInputMode_GameOnly` self)
  (set `self.bShowMouseCursor` false)
  (`/Game/CheekyFPS/UserInterface/WBP_PauseMenu.ClosePauseMenu` (`self.PauseMenuWidget`))
  (set `self.PauseMenuWidget` null)
  (return))

(fn `ShowPauseMenu`
  (`GameplayStatics.SetGamePaused` true)
  (bind _returnvalue (`|CreateWidget` "/Game/CheekyFPS/UserInterface/WBP_PauseMenu.WBP_PauseMenu_C" self))
  (bind _output_get (set `self.PauseMenuWidget` _returnvalue))
  (add `/Game/CheekyFPS/UserInterface/WBP_PauseMenu.OnReturn` _output_get (`|CreateDelegate` :!event `HidePauseMenu`))
  (`UserWidget.AddToViewport` _output_get 0)
  (`WidgetBlueprintLibrary.SetInputMode_UIOnlyEx` self _output_get)
  (set `self.bShowMouseCursor` true)
  (return))

(fn `UserConstructionScript`)