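; Actor component that plays surface-dependent footstep sounds for its owner.
; FootstepCycle accumulates changes in a looping cycle input, ignores the wrap jump, and triggers alternating left and right Walk steps.
; PlayFootstep line-traces from a side-offset position, matches the hit physical material to surface data or a default, and spawns its sound cue with the step type as a parameter.
; A Debug flag shows traces and surface matches.
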(fn `FootstepCycle`
  (params (CycleInput :type "Float (double-precision)"))
  (bind _returnvalue (- (`local.CycleInput`) (`self.LastCycle`)))
  (if (> (`self.NextStep`) 0.25)
    (set `self.NextStep` -0.25)
    (`self.PlayFootstep` "NewEnumerator0" (select `bool` (`self.bWasLastFootstepRight`) :`false` 2))
    (set `self.bWasLastFootstepRight` (not (`self.bWasLastFootstepRight`)))
    (return)
    (else
      (set `self.NextStep` (+ (`self.NextStep`) (select `bool` (> (`KismetMathLibrary.Abs` _returnvalue) 1.0) :`false` _returnvalue)))
      (set `self.LastCycle` (`local.CycleInput`))
      (return))))

(fn `PlayFootstep`
  (params (Type :type "/Game/CheekyFPS/Blueprints/Footsteps/EFootstepTypes Enum" :default "NewEnumerator0") (Position :type Integer :default 1) (OverrideVolume :type "Float (double-precision)" :default 1.0))
  (locals (HitLocation :type "Vector Structure" :default (0.0 0.0 0.0)) (PhysMat :type "PhysicalMaterial Object Reference") (FootstepSurface :type "/Game/CheekyFPS/Blueprints/Footsteps/SFootstepSurface Structure") (bFoundFootstepSurface :type Boolean))
  (bind _returnvalue (`self.GetOwner`))
  (bind _footseperation (`self.FootSeperation`))
  (bind (_footstepsurface_physicalmaterial _footstepsurface_soundcue) (break `/Game/CheekyFPS/Blueprints/Footsteps/SFootstepSurface` (`local.FootstepSurface`)))
  (bind _returnvalue_2 (+ (`SceneComponent.K2_GetComponentLocation` (`Actor.RootComponent` _returnvalue)) (* (`KismetMathLibrary.GetRightVector` (`Actor.K2_GetActorRotation` _returnvalue)) (select `int` (`local.Position`) :`0` (* _footseperation -1.0) :`1` 0.0 :`2` _footseperation))))
  ;[0.09387 1 0.08132] Line Trace - Find out what surface is below the player
  (bind (_outhit _returnvalue_3) (`KismetSystemLibrary.LineTraceSingle` _returnvalue_2 (* _returnvalue_2 (0.0 0.0 -200.0)) "TraceTypeQuery1" false (`|MakeArray` (`self.GetOwner`)) (select `bool` (`self.bDebug`) :`true` "ForDuration" :!type "EDrawDebugTrace Enum")))
  (if _returnvalue_3
    (bind (_bblockinghit _binitialoverlap _time _distance _location _impactpoint _normal _impactnormal _physmat) (`GameplayStatics.BreakHitResult` _outhit))
    (set `local.HitLocation` _location)
    (set `local.PhysMat` _physmat)
    ;[1 0.54 0] Find surface data
    (for _array_element (`self.FootstepSurfaces`)
      (if (== (`.PhysicalMaterial_3_75685D294DC99A767984B9B0C481F84B` (break `/Game/CheekyFPS/Blueprints/Footsteps/SFootstepSurface` _array_element)) (`local.PhysMat`))
        (set `local.FootstepSurface` _array_element)
        (set `local.bFoundFootstepSurface` true)
        ;;[1 0.303 0.4129] Debug
        (if (`self.bDebug`)
          (`KismetSystemLibrary.PrintString` (`KismetStringLibrary.Concat_StrStr` "Found footstep surface data for " (`KismetSystemLibrary.GetDisplayName` (`local.PhysMat`)))))))
    (if (not (`local.bFoundFootstepSurface`))
      (set `local.FootstepSurface` (`self.DefaultFootstepSurface`)))
    (`|ExecutionSequence`
      (:`then_0`
        ;[1 0 0.1066] Play Sound
        (`/Engine/EditorBlueprintResources/StandardMacros.IsValid` _footstepsurface_soundcue
          (:`Is Valid`
            (bind _returnvalue_4 (`GameplayStatics.SpawnSoundAtLocation` _footstepsurface_soundcue (`local.HitLocation`) (struct) (`local.OverrideVolume`) 1.0 0.0 null null))
            (`AudioComponent.SetIntParameter` _returnvalue_4 "FootstepType" (select `/Game/CheekyFPS/Blueprints/Footsteps/EFootstepTypes` (`local.Type`) :`NewEnumerator7` 1 :`NewEnumerator6` 2 :`NewEnumerator2` 3 :`NewEnumerator3` 4 :`NewEnumerator5` 5)))))
      (:`then_1`
        (return)))
    (else
      (return))))