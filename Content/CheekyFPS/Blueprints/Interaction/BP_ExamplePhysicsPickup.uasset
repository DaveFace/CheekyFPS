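; BP_ExamplePhysicsPickup is an example interactable cube the player can pick up, carry, drop and throw.
; CheekyInteractComponent events tint it red on selection and start a grab through the player character's PhysicsHandle.
; While held, Tick follows a camera-relative offset and Pawn collision is ignored.
; HoldStyle chooses whether pressing or releasing Interact drops it; right mouse releases it with a forward impulse.
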(event `self.ReceiveTick`
  (params (DeltaSeconds :type "Float (single-precision)"))
  (bind _returnvalue (`GameplayStatics.GetPlayerCameraManager` 0))
  (bind (_holdoffset_x _holdoffset_y _holdoffset_z) (`KismetMathLibrary.BreakVector` (`self.HoldOffset`)))
  (bind _returnvalue_2 (`PlayerCameraManager.GetCameraRotation` _returnvalue))
  ;[0.958 0.1102 1] Holds the object in front of and just below the player camera
  (`PhysicsHandleComponent.SetTargetLocationAndRotation` (`self.PhysicsHandle`) (+ (`PlayerCameraManager.GetCameraLocation` _returnvalue) (* (`KismetMathLibrary.GetForwardVector` _returnvalue_2) _holdoffset_x) (* (`KismetMathLibrary.GetRightVector` _returnvalue_2) _holdoffset_y) (* (`KismetMathLibrary.GetUpVector` _returnvalue_2) _holdoffset_z)) _returnvalue_2))

(event `self.CheekyInteractComponent.OnBeginSelected`
  ;[1 0.8053 0] Selection Colour
  (if (not (`self.bHoldingItem`))
    (`MaterialInstanceDynamic.SetVectorParameterValue` (`self.MaterialInstance`) "Color" (struct :`R` 1.0 :`A` 1.0))))

(event `self.CheekyInteractComponent.OnEndSelection`
  ;[1 0.8053 0] Selection Colour
  (if (not (`self.bHoldingItem`))
    (`MaterialInstanceDynamic.SetVectorParameterValue` (`self.MaterialInstance`) "Color" (struct :`R` 1.0 :`G` 1.0 :`B` 1.0 :`A` 1.0))))

(event `self.CheekyInteractComponent.OnBeginInteraction`
  (bind _cube (`self.Cube`))
  ;[0.09549 1 0.2229] Pickup
  (bind _output_get (set `self.PhysicsHandle` (`self.GetComponentByClass` (`GameplayStatics.GetPlayerCharacter` 0) "/Script/Engine.PhysicsHandleComponent")))
  (`/Engine/EditorBlueprintResources/StandardMacros.IsValid` _output_get
    (:`Is Valid`
      (set `self.bHoldingItem` true)
      (`PhysicsHandleComponent.GrabComponentAtLocationWithRotation` (`self.PhysicsHandle`) (`self.Cube`) "None" (`PrimitiveComponent.GetCenterOfMass` _cube "None") (`SceneComponent.K2_GetComponentRotation` _cube))
      (`self.SetActorTickEnabled` true)
      (`self.EnableInput` (`GameplayStatics.GetPlayerController` 0))
      (`PrimitiveComponent.SetCollisionResponseToChannel` (`self.Cube`) "ECC_Pawn" "ECR_Ignore")
      (`MaterialInstanceDynamic.SetVectorParameterValue` (`self.MaterialInstance`) "Color" (struct :`R` 1.0 :`G` 1.0 :`B` 1.0 :`A` 1.0)))))

(event `InputAction|[CHEEKY]Interact` :consume false
  (params (Key :type "Key Structure"))
  ;[1 0 0.8797] Release Actions
  (:`Pressed`
    (if (and (`self.bHoldStyle`) (`self.bHoldingItem`))
      (`PhysicsHandleComponent.ReleaseComponent` (`self.PhysicsHandle`) :!label _label)
      (set `self.bHoldingItem` false)
      (`self.SetActorTickEnabled` false)
      (`self.DisableInput` (`GameplayStatics.GetPlayerController` 0))
      (`PrimitiveComponent.SetCollisionResponseToChannel` (`self.Cube`) "ECC_Pawn" "ECR_Block")))
  (:`Released`
    (if (`self.bHoldingItem`)
      (if (not (`self.bHoldStyle`))
        (goto _label)))))

(event `Release`
  ;[1 0 0.8797] Release Actions
  (goto _label))

(event `Key|RightMouseButton`
  (params (Key :type "Key Structure"))
  ;[0.05725 0 1] Throw
  (:`Pressed`
    (if (`self.bHoldingItem`)
      (`self.Release`)
      (`PrimitiveComponent.AddImpulse` (`self.Cube`) (* (`KismetMathLibrary.GetForwardVector` (`PlayerCameraManager.GetCameraRotation` (`GameplayStatics.GetPlayerCameraManager` 0))) (`self.ThrowForce`)) "None" false))))

(fn `UserConstructionScript`
  ;[1 1 1] Create dynamic material instance for the cube
  (bind _returnvalue (`PrimitiveComponent.CreateDynamicMaterialInstance` (`self.Cube`) 0 (`PrimitiveComponent.GetMaterial` (`self.Cube`) 0) "None"))
  (set `self.MaterialInstance` _returnvalue))