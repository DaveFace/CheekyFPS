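; Example interactable cube that demonstrates responses to selection and interaction events from its InteractComponent.
; A timeline scales the cube up when selection begins and reverses when it ends.
; The construction script creates a dynamic material instance with a random colour, which turns a fixed red while interaction lasts and gets a new random colour when it ends.
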(event `self.InteractComponent.OnBeginSelected`
  ;[0.1874 0.2705 1] Scale Up on Selection
  (bind (_direction _animation) (`Timeline|ScaleTimeline` :!label _label)
    (:`Update`
      (`SceneComponent.SetRelativeScale3D` (`self.Cube`) (`KismetMathLibrary.VLerp` (0.5 0.5 0.5) (0.7 0.7 0.7) _animation)))))

(event `self.InteractComponent.OnEndSelection`
  ;[0.1874 0.2705 1] Scale Up on Selection
  (goto _label :!via `Reverse`))

(event `self.InteractComponent.OnBeginInteraction`
  ;[1 0 0.6847] Colour  changes on interaction
  (`MaterialInstanceDynamic.SetVectorParameterValue` (`self.MaterialInstance`) "Color" (struct :`R` 1.0 :`B` 0.099408 :`A` 1.0)))

(event `self.InteractComponent.OnEndInteraction`
  ;[1 0 0.6847] Colour  changes on interaction
  (`self.RandomColour`))

(fn `RandomColour`
  (`MaterialInstanceDynamic.SetVectorParameterValue` (`self.MaterialInstance`) "Color" (make `LinearColor` (`KismetMathLibrary.RandomFloatInRange` 0.0 1.0) (`KismetMathLibrary.RandomFloatInRange` 0.0 1.0) (`KismetMathLibrary.RandomFloatInRange` 0.0 1.0) 1.0))
  (return))

(fn `UserConstructionScript`
  ;[1 1 1] Create dynamic material instance for the cube
  (bind _returnvalue (`PrimitiveComponent.CreateDynamicMaterialInstance` (`self.Cube`) 0 (`PrimitiveComponent.GetMaterial` (`self.Cube`) 0) "None"))
  (set `self.MaterialInstance` _returnvalue)
  (`self.RandomColour`))