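; CheekyInteractComponent is an interaction component in CheekyFPS that tracks whether it is enabled, selected and being interacted with.
; IsSelected stores the selection state and calls the begin-selected or end-selection dispatcher.
; Interaction calls the begin or end interaction dispatcher, then updates IsBeingInteractedWith.
; It has no active BeginPlay or Tick logic, so state changes come through these function calls.
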(fn `Interaction`
  (params (bStart :type Boolean))
  (if bStart
    (`self.OnBeginInteraction`)
    (set `self.bIsBeingInteractedWith` true)
    (return)
    (else
      (`self.OnEndInteraction`)
      (set `self.bIsBeingInteractedWith` false)
      (return))))

(fn `IsEnabled?`
  (returns (bEnabled :type Boolean))
  (return (`self.bEnabled`)))

(fn `IsSelected`
  (params (bIsSelected :type Boolean))
  (bind _output_get (set `self.bIsSelected` bIsSelected))
  (if _output_get
    (`self.OnBeginSelected`)
    (else
      (`self.OnEndSelection`)))
  (return))