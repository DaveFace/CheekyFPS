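; Scene component that finds and drives interactable actors in front of it through their CheekyInteractComponent.
; A looping timer line-traces along its forward vector on Visibility, selecting only enabled interact components.
; Target changes toggle selection and fire begin-selection callbacks, while losing all targets fires lost-selection and ends any active interaction.
; Interact forwards start or stop to the current selection and returns whether one existed.
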(event `self.ReceiveBeginPlay`
  ;[0.1816 0.1744 1] Start trace event
  (`KismetSystemLibrary.K2_SetTimerDelegate` (delegate `TraceEvent`) (`self.TraceInterval`) true))

(event `TraceEvent`
  (bind _currentselectedcomponent (`self.CurrentSelectedComponent`))
  (bind _lastselectedcomponent (`self.LastSelectedComponent`))
  ;[0 0.4442 1] Perform trace
  (set `self.LastSelectedComponent` (`self.CurrentSelectedComponent`))
  (bind _result (`self.Trace`))
  (bind _output_get (set `self.CurrentSelectedComponent` _result))
  (`/Engine/EditorBlueprintResources/StandardMacros.IsValid` _output_get
    (:`Is Valid`
      (set `self.bValidTarget` true)
      (`/Engine/EditorBlueprintResources/StandardMacros.IsValid` (`self.LastSelectedComponent`)
        (:`Is Valid`
          ;[0.01239 1 0.3792] If there was a different actor selected last, then deselect it first
          ; (If current = last, then we're still selecting the same actor, and don't need to do anything)
          (if (not (== (`self.CurrentSelectedComponent`) (`self.LastSelectedComponent`)))
            (`/Game/CheekyFPS/Blueprints/Interaction/CheekyInteractComponent.IsSelected` (`self.LastSelectedComponent`) false)
            ;[0 0.291 1 1 28] Select the new actor
            (`/Game/CheekyFPS/Blueprints/Interaction/CheekyInteractComponent.IsSelected` _currentselectedcomponent true :!label _label)
            (`self.OnBeginSelection` (`self.GetOwner` _currentselectedcomponent))))
        (:`Is Not Valid`
          (goto _label))))
    (:`Is Not Valid`
      ;[1 0.1254 0] Lost selection
      (set `self.bValidTarget` false)
      (`/Engine/EditorBlueprintResources/StandardMacros.IsValid` _lastselectedcomponent
        (:`Is Valid`
          (`/Game/CheekyFPS/Blueprints/Interaction/CheekyInteractComponent.IsSelected` _lastselectedcomponent false)
          (`self.OnLostSelection` (`self.GetOwner` _lastselectedcomponent))
          ;[1 0.7589 0] If we were interacting, stop now that we've lost the target
          (if (`self.bIsInteracting`)
            (`/Game/CheekyFPS/Blueprints/Interaction/CheekyInteractComponent.Interaction` (`self.LastSelectedComponent`) false)
            (set `self.bIsInteracting` false)))))))

(fn `Interact`
  (params (bStart :type Boolean))
  (returns (bSuccessful :type Boolean))
  (`/Engine/EditorBlueprintResources/StandardMacros.IsValid` (`self.CurrentSelectedComponent`)
    (:`Is Valid`
      (`/Game/CheekyFPS/Blueprints/Interaction/CheekyInteractComponent.Interaction` (`self.CurrentSelectedComponent`) (`local.bStart`))
      (set `self.bIsInteracting` (`local.bStart`))
      (return true))
    (:`Is Not Valid`
      (return false))))

(fn `Trace`
  (returns (Result :type "/Game/CheekyFPS/Blueprints/Interaction/CheekyInteractComponent Object Reference"))
  (bind _returnvalue (`self.K2_GetComponentLocation`))
  ;[1 0.0625 0.0625] Line Trace
  (bind (_outhit _returnvalue_2) (`KismetSystemLibrary.LineTraceSingle` _returnvalue (+ _returnvalue (* (`self.GetForwardVector`) (`self.InteractionRange`))) "TraceTypeQuery1" true (`|MakeArray` (`self.GetOwner`)) (select `bool` (`self.DrawDebugTrace`) :`true` "ForDuration" :!type "EDrawDebugTrace Enum") true (struct :`R` 1.0 :`A` 1.0) (struct :`G` 1.0 :`A` 1.0) 1.0))
  (if _returnvalue_2
    (bind (_bblockinghit _binitialoverlap _time _distance _location _impactpoint _normal _impactnormal _physmat _hitactor) (`GameplayStatics.BreakHitResult` _outhit))
    ;[0.01289 1 0.2456] Is this something we can interact with?
    (`/Engine/EditorBlueprintResources/StandardMacros.IsValid` _hitactor ; Because not everything we hit will be an actor
      (:`Is Valid`
        (bind _returnvalue_3 (`Actor.GetComponentByClass` _hitactor "/Game/CheekyFPS/Blueprints/Interaction/CheekyInteractComponent.CheekyInteractComponent_C"))
        (`/Engine/EditorBlueprintResources/StandardMacros.IsValid` _returnvalue_3
          (:`Is Valid`
            (if (`/Game/CheekyFPS/Blueprints/Interaction/CheekyInteractComponent.IsEnabled?` _returnvalue_3)
              (return _returnvalue_3)
              (else
                _)))
          (:`Is Not Valid`
            _)))
      (:`Is Not Valid`
        _)))
  (return null))