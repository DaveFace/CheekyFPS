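; SaveGame_CheekyConfig is the save game object for CheekyFPS look settings, covering inversion, sensitivity and smoothing for mouse and gamepad.
; Getter functions take an IsGamepad flag and return the matching device's value, with separate X and Y axes for inversion and sensitivity.
; GetLookSmooth converts the stored smoothing amount into an interp speed, lowering it from a fixed maximum so higher smoothing means slower interpolation.
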(fn `GetLookInvertX`
  (params (bIsGamepad :type Boolean))
  (returns (bInvertX :type Boolean))
  (return (select `bool` bIsGamepad :`false` (`self.bInvertMouseX`) :`true` (`self.bInvertGamepadX`))))

(fn `GetLookInvertY`
  (params (bIsGamepad :type Boolean))
  (returns (bInvertY :type Boolean))
  (return (select `bool` bIsGamepad :`false` (`self.bInvertMouseY`) :`true` (`self.bInvertGamepadY`))))

(fn `GetLookSensX`
  (params (bIsGamepad :type Boolean))
  (returns (LookSensX :type "Float (double-precision)"))
  (return (select `bool` bIsGamepad :`false` (`self.MouseSensX`) :`true` (`self.GamepadSensX`))))

(fn `GetLookSensY`
  (params (bIsGamepad :type Boolean))
  (returns (LookSensY :type "Float (double-precision)"))
  (return (select `bool` bIsGamepad :`false` (`self.MouseSensY`) :`true` (`self.GamepadSensY`))))

(fn `GetLookSmooth`
  (params (bIsGamepad :type Boolean))
  (returns (LookSmooth :type "Float (double-precision)"))
  (return (- 50.0 (* (select `bool` bIsGamepad :`false` (`self.MouseSmooth`) :`true` (`self.GamepadSmooth`)) 30.0))))