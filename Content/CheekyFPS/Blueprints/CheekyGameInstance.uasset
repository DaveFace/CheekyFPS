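; Game instance for CheekyFPS that owns the persistent game config, stored as a SaveGame_CheekyConfig in a save slot.
; On Init it loads the slot into GameConfigSave; if that fails, it writes a new default config and calls LoadConfig again recursively.
; SaveConfig writes the cached config back to the same slot, and failed saves are reported through printed messages.
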(event `self.ReceiveInit`
  (`self.LoadConfig`))

(fn `LoadConfig`
  (bind _returnvalue (`GameplayStatics.LoadGameFromSlot` (`self.GameConfigString`)))
  (bind _assave_game_cheeky_config (cast `/Game/CheekyFPS/Blueprints/SaveGame/SaveGame_CheekyConfig` _returnvalue)
    (:`then`
      (set `self.GameConfigSave` _assave_game_cheeky_config)
      (return))
    (:`CastFailed`
      ;[0 0.9245 1] No config file exists - create a new one using defaults
      (bind _returnvalue_2 (`GameplayStatics.CreateSaveGameObject` "/Game/CheekyFPS/Blueprints/SaveGame/SaveGame_CheekyConfig.SaveGame_CheekyConfig_C"))
      (bind _returnvalue_3 (`GameplayStatics.SaveGameToSlot` _returnvalue_2 (`self.GameConfigString`)))
      (if _returnvalue_3
        (`KismetSystemLibrary.PrintString` "No config file found - creating one")
        (`self.LoadConfig`)
        (return)
        (else
          (`KismetSystemLibrary.PrintString` "Failed to create a default config file")
          (return))))))

(fn `SaveConfig`
  (bind _returnvalue (`GameplayStatics.SaveGameToSlot` (`self.GameConfigSave`) (`self.GameConfigString`)))
  (if _returnvalue
    (return)
    (else
      (`KismetSystemLibrary.PrintString` "Failed to save settings to disk.")
      (return))))