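; Actor component for level communication that passes name and float signals from its owner to other actors.
; Send functions find the same component on the target and call its OnNameSignal or OnFloatSignal dispatcher with the owner as sender.
; SendNameArray sends a batch of target and message pairs through SendName.
; Targets lacking a valid transceiver trigger a printed error naming the signal and target.
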(fn `PrintError`
  (params (Target :type "Actor Object Reference") (SignalType :type String) (SignalValue :type String))
  (`KismetSystemLibrary.PrintString` (`KismetStringLibrary.Concat_StrStr` (`KismetSystemLibrary.GetDisplayName` self) " tried to send signal \"" (`local.SignalValue`) "\" of type " (`local.SignalType`) ", but failed because" (`KismetSystemLibrary.GetDisplayName` (`local.Target`)) "does not have a valid signal transciever component."))
  (return))

(fn `SendFloat`
  (params (Target :type "Actor Object Reference") (Float :type "Float (double-precision)"))
  (bind _returnvalue (`Actor.GetComponentByClass` Target "SignalTranscieverComponent_C"))
  (`/Engine/EditorBlueprintResources/StandardMacros.IsValid` _returnvalue
    (:`Is Valid`
      (`self.OnFloatSignal` _returnvalue (`self.GetOwner`) (`local.Float`))
      (return))
    (:`Is Not Valid`
      (`self.PrintError` (`local.Target`) "Float" (`KismetStringLibrary.Conv_DoubleToString` (`local.Float`)))
      (return))))

(fn `SendName`
  (params (NamePair :type "/Game/CheekyFPS/Blueprints/LevelCommunication/SNameSignalPair Structure"))
  (bind (_message _target) (break `/Game/CheekyFPS/Blueprints/LevelCommunication/SNameSignalPair` NamePair))
  (bind _returnvalue (`Actor.GetComponentByClass` _target "SignalTranscieverComponent_C"))
  (`/Engine/EditorBlueprintResources/StandardMacros.IsValid` _returnvalue
    (:`Is Valid`
      (`self.OnNameSignal` _returnvalue (`self.GetOwner`) _message)
      (return))
    (:`Is Not Valid`
      (`self.PrintError` _target "Name" (`KismetStringLibrary.Conv_NameToString` _message))
      (return))))

(fn `SendNameArray`
  (params (Name :type "Array of /Game/CheekyFPS/Blueprints/LevelCommunication/SNameSignalPair Structure"))
  (for _array_element Name
    (`self.SendName` _array_element))
  (return))