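; LeanComponent is a scene component for a Character that adds side-to-side leaning by offsetting and rolling itself from an axis input.
; CalculateLean sphere-traces sideways to limit lean near obstacles, scales it down when moving or crouched, and zeroes it when not on the ground.
; The smoothed signed alpha, interpolated more slowly when input is released, drives lateral offset, vertical shift and roll in UpdateLeanFromAxis.
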(event `self.ReceiveBeginPlay`
  ;[1 0.3245 0.6236] Check we're on a character actor
  (bind _ascharacter (cast `Character` (`self.GetOwner`))
    (:`then`
      (set `self.PlayerCharacter` _ascharacter))
    (:`CastFailed`
      (`KismetSystemLibrary.PrintString` "LeanComponent should only be attached to a character actor"))))

(fn `CalculateLean`
  (params (Axis :type "Float (double-precision)"))
  (locals (TraceResult :type "Float (double-precision)") (LeanBuffer :type "Float (double-precision)" :default 15.0))
  (bind _returnvalue (+ (`self.K2_GetComponentLocation` self) (0.0 0.0 0.0)))
  ;[0.04342 0.3883 1] Trace to check available space at camera level
  (bind (_outhit _returnvalue_2) (`KismetSystemLibrary.SphereTraceSingle` _returnvalue (+ _returnvalue (* (`self.GetRightVector` self) (* (`local.Axis`) (- (`self.LeanDist`) (`local.LeanBuffer`))))) 25.0 "TraceTypeQuery1" false (`|MakeArray` (`self.PlayerCharacter`) :!type "Actor Object Reference")))
  ;[1 0.02924 0.566] If we hit something, return a normalised value of the distance
  (if _returnvalue_2
    (set `local.TraceResult` (`KismetMathLibrary.FClamp` (/ (`.Distance` (`GameplayStatics.BreakHitResult` _outhit)) (- (`self.LeanDist`) (`local.LeanBuffer`)))))
    (else
      ;[0.07549 0.1296 1] If we didn't hit anything, just return 1 (max lean)
      (set `local.TraceResult` 1.0)))
  ;[1 0.2618 0] Generate a smooth, normalised (-1 to 1) value for the lean
  (set `self.SmoothLeanAlpha` (`KismetMathLibrary.FInterpTo` (`self.SmoothLeanAlpha`) (* (`local.TraceResult`) (`local.Axis`) (`KismetMathLibrary.FClamp` (- 1.0 (/ (`KismetMathLibrary.VSize` (`CharacterMovementComponent.GetLastUpdateVelocity` (`Character.CharacterMovement` (`self.PlayerCharacter`)))) 500.0)) 0.4) (select `bool` (`NavMovementComponent.IsCrouching` (`Character.CharacterMovement` (`self.PlayerCharacter`))) :`false` 1.0 :`true` 0.7 :!type "Float (single-precision)") (`KismetMathLibrary.Conv_BoolToDouble` (`NavMovementComponent.IsMovingOnGround` (`Character.CharacterMovement` (`self.PlayerCharacter`))))) (`GameplayStatics.GetWorldDeltaSeconds`) (select `bool` (`KismetMathLibrary.NearlyEqual_FloatFloat` (`local.Axis`) 0.0 0.001) :`false` 15.0 :`true` 5.0 :!type "Float (single-precision)")))
  (return))

(fn `UpdateLeanFromAxis`
  (params (Axis :type "Float (double-precision)"))
  (`self.CalculateLean` Axis)
  (`self.K2_SetRelativeLocationAndRotation` (+ (`KismetMathLibrary.MakeVector` 0.0 (* (`self.LeanDist`) (`self.SmoothLeanAlpha`))) (`KismetMathLibrary.MakeVector` 0.0 0.0 (* (`self.LeanVerticalShift`) (`KismetMathLibrary.Abs` (`self.SmoothLeanAlpha`))))) (`KismetMathLibrary.MakeRotator` (* (`self.LeanRotation`) (`self.SmoothLeanAlpha`))))
  (return))