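; Player settings manager for CheekyFPS that serves look settings for mouse and gamepad input.
; Getter functions take an IsGamepad flag and return the matching sensitivity, axis inversion or smoothing value, with no active event logic.
; GetLookSmooth remaps the stored value inversely, so a higher smoothing setting returns a lower number.
; GetLookSensX returns the mouse Y sensitivity for mouse input, so no separate mouse X value is used.
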(fn `GetLookInvertX`
  (params (bIsGamepad :type Boolean))
  (returns (bInvertX :type Boolean))
  (return (select `bool` bIsGamepad :`false` (`self.bInvertMouseX`) :`true` (`self.bInvertGamepadX`))))

(fn `GetLookInvertY`
  (params (bIsGamepad :type Boolean))
  (returns (bInvertY :type Boolean))
  (return (select `bool` bIsGamepad :`false` (`self.bInvertMouseY`) :`true` (`self.bInvertGamepadY`))))

(fn `GetLookSensX`
  (params (bIsGamepad :type Boolean))
  (returns (LookSensX :type "Float (double-precision)"))
  (return (select `bool` bIsGamepad :`false` (`self.MouseSensY`) :`true` (`self.GamepadSensX`))))

(fn `GetLookSensY`
  (params (bIsGamepad :type Boolean))
  (returns (LookSensY :type "Float (double-precision)"))
  (return (select `bool` bIsGamepad :`false` (`self.MouseSensY`) :`true` (`self.GamepadSensY`))))

(fn `GetLookSmooth`
  (params (bIsGamepad :type Boolean))
  (returns (Smooth :type "Float (double-precision)"))
  (return (- 50.0 (* (select `bool` bIsGamepad :`false` (`self.MouseSmooth`) :`true` (`self.GamepadSmooth`)) 20.0))))