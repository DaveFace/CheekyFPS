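; Parkour component for a Character that decides on a jump action whether to vault or mantle an obstacle.
; MantleTrace finds a wall within a speed-scaled distance, blends facing with the wall normal, then traces for ledge, clearance, far-side drop and headroom, optionally mantling into crouch.
; JumpAction passes the resulting locations and rotation to PerformVault or PerformMantle, which are empty events here, and returns whether either fired.
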(event `self.ReceiveBeginPlay`
  ;[1 0 0.9088] Beginplay Stuff
  (bind _ascharacter (cast `Character` (`self.GetOwner`)))
  (bind _output_get (set `self.PlayerCharacter` _ascharacter))
  (set `self.PlayerController` (`Pawn.GetController` _output_get)))

(event `PerformVault`
  (params (LocationA :type "Vector Structure") (LocationB :type "Vector Structure") (Rotation :type "Rotator Structure")))

(event `PerformMantle`
  (params (LocationA :type "Vector Structure") (LocationB :type "Vector Structure") (Rotation :type "Rotator Structure") (bIntoCrouch :type Boolean)))

(fn `FlattenNormal`
  (params (In :type "Vector Structure"))
  (returns (Out :type "Vector Structure"))
  (return (`KismetMathLibrary.MakeVector` (.x In) (.y In))))

(fn `IsPerformingAction`
  (returns (bIsParkouring :type Boolean))
  (return (`self.bIsParkouring`)))

(fn `JumpAction`
  (returns (bParkourActionPerformed :type Boolean))
  (bind (_bcanvault _bcanmantle _bcrouch _locationa _locationb _ledgerotation) (`self.MantleTrace` false))
  (if (and _bcanvault (`self.bEnableVaulting`))
    (`self.PerformVault` _locationa _locationb _ledgerotation)
    (return true)
    (elif (and _bcanmantle (`self.bEnableMantle`))
      (`self.PerformMantle` _locationa _locationb _ledgerotation _bcrouch)
      (return true)
      (else
        (return false)))))

(fn `MantleTrace`
  (params (bDrawDebug :type Boolean))
  (returns (bCanVault :type Boolean) (bCanMantle :type Boolean) (bCrouch :type Boolean) (LocationA :type "Vector Structure") (LocationB :type "Vector Structure") (LedgeRotation :type "Rotator Structure"))
  (locals (DebugTraces :type "EDrawDebugTrace Enum" :default "None") (ActorsIgnore :type "Array of Actor Object Reference") (Capsule :type "CapsuleComponent Object Reference") (PlayerHalfHeight :type "Float (double-precision)") (WallHit :type "HitResult Structure") (VaultCheckHit :type "HitResult Structure") (VaultTraceEndLoc :type "Vector Structure" :default (0.0 0.0 0.0)) (VaultTraceStartLoc :type "Vector Structure" :default (0.0 0.0 0.0)) (VaultNormal :type "Vector Structure" :default (0.0 0.0 0.0)) (bShouldPlayerCrouch :type Boolean) (LedgeLoc :type "Vector Structure" :default (0.0 0.0 0.0)))
  (bind _capsule (`local.Capsule`))
  (bind _vaulttraceendloc (`local.VaultTraceEndLoc`))
  (bind _returnvalue (`SceneComponent.K2_GetComponentLocation` _capsule))
  (bind _returnvalue_2 (`SceneComponent.K2_GetComponentRotation` _capsule))
  (bind _returnvalue_3 (+ (`.Location` (`GameplayStatics.BreakHitResult` (`local.WallHit`))) (* (`local.VaultNormal`) 20.0)))
  ;[0.149 1 0] Boilerplate - we use these values a lot, so easier to set them upfront
  (set `local.ActorsIgnore` (`|MakeArray` (`self.PlayerCharacter`) :!type "Actor Object Reference"))
  (set `local.DebugTraces` (select `bool` (`local.bDrawDebug`) :`true` "ForDuration" :!type "EDrawDebugTrace Enum"))
  (bind _output_get (set `local.Capsule` (`Character.CapsuleComponent` (`self.PlayerCharacter`))))
  (set `local.PlayerHalfHeight` (`CapsuleComponent.CapsuleHalfHeight` _output_get))
  (`|ExecutionSequence`
    (:`then_0`
      ;[0.02446 1 0] Check if there is a wall in front of the player
      (bind (_outhit _returnvalue_4) (`KismetSystemLibrary.BoxTraceSingle` _returnvalue (+ _returnvalue (* (`self.FlattenNormal` (`KismetMathLibrary.GetForwardVector` _returnvalue_2)) (`self.WallDistance`))) (1.0 1.0 50.0) (`KismetMathLibrary.MakeRotator` (.roll _returnvalue_2) 0.0 (.yaw _returnvalue_2)) "TraceTypeQuery1" false (`local.ActorsIgnore`) (`local.DebugTraces`)))
      (if _returnvalue_4
        (set `local.WallHit` _outhit)
        ;[0.7896 1 0] Calculate our vault direction (mix between player direction, and the wall normal)
        (set `local.VaultNormal` (`self.FlattenNormal` (`KismetMathLibrary.VLerp` (`KismetMathLibrary.GetForwardVector` (`SceneComponent.K2_GetComponentRotation` (`local.Capsule`))) (* (`.Normal` (`GameplayStatics.BreakHitResult` (`local.WallHit`))) -1.0) 0.7)))
        ;[1 0.2996 0] Detect if there is a ledge, and how high it is
        (bind (_outhit_2 _returnvalue_5) (`KismetSystemLibrary.LineTraceSingle` (+ _returnvalue_3 (`KismetMathLibrary.MakeVector` 0.0 0.0 (`self.HeightClear`))) (- _returnvalue_3 (0.0 0.0 10.0)) "TraceTypeQuery1" false (`local.ActorsIgnore`) (`local.DebugTraces`)))
        (if _returnvalue_5
          (set `local.LedgeLoc` (+ (`.Location` (`GameplayStatics.BreakHitResult` _outhit_2)) (0.0 0.0 1.0)))
          (else
            (return false false false (0.0 0.0 0.0) (0.0 0.0 0.0)) ; No valid ledge (Either there's a wall, or the ledge\nis so low we can just jump over it)
          ))
        (else
          (return false false false (0.0 0.0 0.0) (0.0 0.0 0.0)) ; There's no wall to climb / vault
        )))
    (:`then_1`
      ;[1 0.01091 0] Check if we can clear the wall
      (bind _output_get_2 (set `local.VaultTraceStartLoc` (+ (`local.LedgeLoc`) (0.0 0.0 50.0))))
      (set `local.VaultTraceEndLoc` (+ _output_get_2 (* (`local.VaultNormal`) 100.0)))
      (bind (_outhit_3 _returnvalue_6) (`KismetSystemLibrary.BoxTraceSingle` (`local.VaultTraceStartLoc`) (`local.VaultTraceEndLoc`) (0.0 40.0 50.0) (`KismetMathLibrary.MakeRotFromX` (`local.VaultNormal`)) "TraceTypeQuery1" false (`local.ActorsIgnore`) (`local.DebugTraces`)))
      (if _returnvalue_6
        (set `local.VaultCheckHit` _outhit_3)
        ;[1 0 0.2361] If we hit something, did we at least trace far enough to mantle up?
        (if (not (> (`.Distance` (`GameplayStatics.BreakHitResult` (`local.VaultCheckHit`))) 50.0))
          (return false false false (0.0 0.0 0.0) (0.0 0.0 0.0)) ; No space to mantle
        )
        (else
          ;[1 0 0.6562] Is there a drop the other side of the wall?
          (bind (_outhit_4 _returnvalue_7) (`KismetSystemLibrary.SphereTraceSingle` _vaulttraceendloc (- _vaulttraceendloc (`KismetMathLibrary.MakeVector` 0.0 0.0 (`local.PlayerHalfHeight`))) 30.0 "TraceTypeQuery1" false (`local.ActorsIgnore`) (`local.DebugTraces`) true (struct :`R` 1.0 :`G` 0.833041 :`A` 1.0)))
          (if (not _returnvalue_7)
            ;[0.3505 0 1] Vault
            (return true false false (+ (`local.LedgeLoc`) (0.0 0.0 50.0)) (`local.VaultTraceEndLoc`) (`KismetMathLibrary.MakeRotFromX` (`local.VaultNormal`))) ; Player has a clear path over the wall, and\nspace to drop the other side
          ))))
    (:`then_2`
      ;[0.04996 0 1] Is there space to stand on the ledge?
      (bind (_outhit_5 _returnvalue_8) (`KismetSystemLibrary.BoxTraceSingle` (`local.LedgeLoc`) (+ (`local.LedgeLoc`) (`KismetMathLibrary.MakeVector` 0.0 0.0 (* (`local.PlayerHalfHeight`) 2.0))) (20.0 20.0 0.0) (struct) "TraceTypeQuery1" false (`local.ActorsIgnore`) (`local.DebugTraces`)))
      ;[0 0.7593 1] Determine if we can mantle and/or we need to change stance to do it
      (if _returnvalue_8
        (if (and (> (`.Distance` (`GameplayStatics.BreakHitResult` _outhit_5)) (`self.CrouchHeight`)) (`self.bEnableMantleIntoCrouch`))
          (set `local.bShouldPlayerCrouch` true)
          (else
            (return false false false (0.0 0.0 0.0) (0.0 0.0 0.0)) ; Can't mantle as there's no space to stand up
          ))
        (else
          (set `local.bShouldPlayerCrouch` false)))
      ;[0.02376 0 1] Mantle
      (return false true (`local.bShouldPlayerCrouch`) (+ (`local.LedgeLoc`) (* (`local.VaultNormal`) -50.0) (0.0 0.0 20.0)) (+ (`local.LedgeLoc`) (`KismetMathLibrary.MakeVector` 0.0 0.0 (select `bool` (`local.bShouldPlayerCrouch`) :`false` (`local.PlayerHalfHeight`) :`true` (`self.CrouchHeight`)))) (`KismetMathLibrary.MakeRotFromX` (`local.VaultNormal`))) ; Mantle
    )))

(fn `WallDistance`
  (returns (WallDistance :type "Float (double-precision)"))
  (return (`KismetMathLibrary.Lerp` (`self.WallDistanceMin`) (`self.WallDistanceMax`) (`KismetMathLibrary.FClamp` (/ (`KismetMathLibrary.VSizeXY` (`CharacterMovementComponent.GetLastUpdateVelocity` (`Character.CharacterMovement` (`self.PlayerCharacter`)))) 500.0)))))