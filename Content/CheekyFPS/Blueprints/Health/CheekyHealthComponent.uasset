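; Actor component that gives its owner health, with damage, death notification, optional regeneration and fall damage for Characters.
; It binds to the owner's any-damage event, clamps and rounds HP on every change, and fires a death dispatcher at zero.
; Non-lethal damage restarts a retriggerable delay, then a looping timer heals until full.
; OnLanded maps impact speed through a curve and applies the result as standard damage.
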(event `self.ReceiveBeginPlay`
  (bind _returnvalue (`self.GetOwner`))
  ;[0.9737 0 1] Beginplay Stuff
  (add `Actor.OnTakeAnyDamage` _returnvalue (`|CreateDelegate` :!event `OnTakeAnyDamage`))
  (bind _ascharacter (cast `Character` _returnvalue)
    (:`then`
      (set `self.Character` _ascharacter)
      (set `self.bIsCharacter` true))
    (:`CastFailed`
      (set `self.bIsCharacter` false))))

(event `RegenHealth`
  ;[1 0.7974 0] Health Regeneration
  (`KismetSystemLibrary.K2_ClearTimer` null "RegenerateHealth") ; Make sure timer isn't running\nE.g. if the timer was running, and player\ntakes damage and triggers this event again\nthen stop regenerating
  (`KismetSystemLibrary.RetriggerableDelay` (`self.RegenerateDelay`))
  (`KismetSystemLibrary.K2_SetTimer` null "RegenerateHealth" 0.1 true))

(fn `AddHealth`
  (params (HealthAdd :type "Float (double-precision)"))
  (set `self.CurrentHP` (`KismetMathLibrary.Conv_IntToDouble` (`KismetMathLibrary.Round` (`KismetMathLibrary.FClamp` (+ (`self.CurrentHP`) (`local.HealthAdd`)) 0.0 (`self.MaxHP`)))))
  (return))

(fn `GetHealth`
  (returns (CurrentHP :type "Float (double-precision)") (MaxHP :type "Float (double-precision)"))
  (return (`self.CurrentHP`) (`self.MaxHP`)))

(fn `OnLanded`
  (params (VelocityOnImpact :type "Float (double-precision)"))
  (locals (Damage :type "Float (double-precision)"))
  (bind _character (`self.Character`))
  (if (`self.bIsCharacter`)
    (bind _output_get (set `local.Damage` (`CurveFloat.GetFloatValue` (`self.FallDamage`) (`KismetMathLibrary.Abs` (`local.VelocityOnImpact`)))))
    (if (== _output_get 0.0)
      (return)
      (else
        (`GameplayStatics.ApplyDamage` _character (`local.Damage`) null _character)
        (return)))
    (else
      ;[1 0.1073 0.02767] Error
      (`KismetSystemLibrary.PrintString` "(CheekyHealthComponent) OnLanded only works for Characters!")
      (return))))

(fn `OnTakeAnyDamage`
  (params (DamagedActor :type "Actor Object Reference") (Damage :type "Float (double-precision)") (DamageType :type "DamageType Object Reference") (InstigatedBy :type "Controller Object Reference") (DamageCauser :type "Actor Object Reference"))
  (`self.RemoveHealth` Damage)
  (return))

(fn `RegenerateHealth`
  (`self.AddHealth` (/ (`self.RegenerateSpeed`) 10.0))
  ;[0.2842 0.2266 1] If we've healed the player, stop this running
  (if (== (`self.CurrentHP`) (`self.MaxHP`))
    (`KismetSystemLibrary.K2_ClearTimer` null "RegenerateHealth"))
  (return))

(fn `RemoveHealth`
  (params (HealthLost :type "Float (double-precision)"))
  (bind _output_get (set `self.CurrentHP` (`KismetMathLibrary.Conv_IntToDouble` (`KismetMathLibrary.Round` (`KismetMathLibrary.FClamp` (- (`self.CurrentHP`) (`local.HealthLost`)) 0.0 (`self.MaxHP`))))))
  (if (== _output_get 0.0)
    (`self.OnThingDead`)
    (return)
    (else
      ;[0.1277 0.2754 1] Regenerate Health (If Enabled)
      (if (and (< _output_get (`self.MaxHP`)) (`self.bRegenerateHealth`))
        (`self.RegenHealth`))
      (return))))