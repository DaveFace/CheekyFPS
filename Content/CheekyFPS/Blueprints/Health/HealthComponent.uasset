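; Health component that tracks HP for its owning actor and adds fall damage for Characters.
; It binds to the owner's any-damage event, subtracts damage as clamped, rounded HP, and broadcasts OnThingDead at zero.
; OnLanded converts vertical landing speed through the FallDamage curve, routes nonzero results through ApplyDamage, and broadcasts OnLandFootstep with a stronger value for damaging landings.
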(event `self.ReceiveBeginPlay`
  (bind _returnvalue (`self.GetOwner`))
  (add `Actor.OnTakeAnyDamage` _returnvalue (`|CreateDelegate` :!event `OnTakeAnyDamage`))
  (bind _ascharacter (cast `Character` _returnvalue)
    (:`then`
      (set `self.Character` _ascharacter)
      (set `self.bIsCharacter` true))
    (:`CastFailed`
      (set `self.bIsCharacter` false))))

(fn `AddHealth`
  (params (HealthAdd :type "Float (double-precision)"))
  (set `self.CurrentHP` (`KismetMathLibrary.Conv_IntToDouble` (`KismetMathLibrary.Round` (`KismetMathLibrary.FClamp` (+ (`self.CurrentHP`) (`local.HealthAdd`)) 0.0 (`self.MaxHP`)))))
  (return))

(fn `GetHealth`
  (returns (CurrentHP :type "Float (double-precision)") (MaxHP :type "Float (double-precision)"))
  (return (`self.CurrentHP`) (`self.MaxHP`)))

(fn `OnLanded`
  (locals (Damage :type "Float (double-precision)"))
  (bind _character (`self.Character`))
  (bind _output_get (set `local.Damage` (`CurveFloat.GetFloatValue` (`self.FallDamage`) (`KismetMathLibrary.Abs` (.z (`CharacterMovementComponent.GetLastUpdateVelocity` (`Character.CharacterMovement` (`self.Character`))))))))
  (if (== _output_get 0.0)
    (`self.OnLandFootstep` 0.5)
    (return)
    (else
      (`GameplayStatics.ApplyDamage` _character (`local.Damage`) null _character)
      (`self.OnLandFootstep` 1.0)
      (return))))

(fn `OnTakeAnyDamage`
  (params (DamagedActor :type "Actor Object Reference") (Damage :type "Float (double-precision)") (DamageType :type "DamageType Object Reference") (InstigatedBy :type "Controller Object Reference") (DamageCauser :type "Actor Object Reference"))
  (`self.RemoveHealth` Damage)
  (return))

(fn `RemoveHealth`
  (params (HealthLost :type "Float (double-precision)"))
  (bind _output_get (set `self.CurrentHP` (`KismetMathLibrary.Conv_IntToDouble` (`KismetMathLibrary.Round` (`KismetMathLibrary.FClamp` (- (`self.CurrentHP`) (`local.HealthLost`)) 0.0 (`self.MaxHP`))))))
  (if (== _output_get 0.0)
    (`self.OnThingDead`))
  (return))